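; Cannonball Blueprint for Warehouse Wreckage, with a Launch function that fires its static mesh along the actor's forward vector using a fixed velocity-change impulse.
; It also holds small helper functions to decrement, check and print an Ammo count, and to print welcome messages.
; SpawnProjectile and the construction script are empty, and no event or function here calls any of these functions.
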(fn `DecreaseAmmo`
  (set `self.Ammo` (- (`self.Ammo`) 1)))

(fn `Has Ammo?`
  (returns (ReturnValue :type Boolean))
  (return (> (`self.Ammo`) 0)))

(fn `Launch`
  (`PrimitiveComponent.AddImpulse` (`self.StaticMeshComponent`) (* (`self.GetActorForwardVector`) 6000) "None" true))

(fn `PrintAmmo`
  (`KismetSystemLibrary.PrintString` (`KismetStringLibrary.Conv_IntToString` (`self.Ammo`))))

(fn `PrintWelcomeMessages`
  (`KismetSystemLibrary.PrintString` "Welcome to Warehouse Wreckage!")
  (`KismetSystemLibrary.PrintString` "Get ready to rumble!"))

(fn `SpawnProjectile`)

(fn `UserConstructionScript`)